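; Actor whose mesh fades out and back in through a timeline-driven "Fade" material parameter.
; Construction caches the original materials and builds dynamic instances from the fade materials.
; FadeOut swaps in those instances and plays the timeline; Fadein reverses it.
; On finish, a value of one or more restores materials and blocking, while lower non-negative values ignore a custom trace channel, plus Visibility if BlockVisibility is set.
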(event `self.ReceiveBeginPlay`)

(event `/Game/Blueprints/Actors/FadeActor/BPI_Fade.FadeOut`
  (`self.SetMaterialToDynamicInstances`)
  (bind (_direction _fade) (`Timeline|FadeTimeline` :!label _label)
    (:`Update`
      (for _array_element (`self.Dynamic Material Instance`)
        (`MaterialInstanceDynamic.SetScalarParameterValue` _array_element "Fade" _fade)))
    (:`Finished`
      (`self.FadeFinished` _fade))))

(event `/Game/Blueprints/Actors/FadeActor/BPI_Fade.FadeIn`
  (goto _label :!via `Reverse`))

(fn `FadeFinished`
  (params (FadedValue :type "Float (single-precision)"))
  (if (>= FadedValue 1.0)
    (`self.ResetMaterials`)
    (`PrimitiveComponent.SetCollisionResponseToChannel` (`self.Mesh`) "ECC_GameTraceChannel2" "ECR_Block")
    (if (`self.BlockVisibility`)
      (`PrimitiveComponent.SetCollisionResponseToChannel` (`self.Mesh`) "ECC_Visibility" "ECR_Block"))
    (elif (>= FadedValue 0.0)
      (`PrimitiveComponent.SetCollisionResponseToChannel` (`self.Mesh`) "ECC_GameTraceChannel2" "ECR_Ignore")
      (if (`self.BlockVisibility`)
        (`PrimitiveComponent.SetCollisionResponseToChannel` (`self.Mesh`) "ECC_Visibility" "ECR_Ignore")))))

(fn `ResetMaterials`
  (for (_array_element _array_index) (`self.OriginalMaterials`)
    (`PrimitiveComponent.SetMaterial` (`self.Mesh`) _array_index _array_element)))

(fn `SetMaterialToDynamicInstances`
  (for (_array_element _array_index) (`self.Dynamic Material Instance`)
    (`PrimitiveComponent.SetMaterial` (`self.Mesh`) _array_index _array_element)))

(fn `UserConstructionScript`
  (`KismetArrayLibrary.Array_Clear` (`self.Dynamic Material Instance`))
  (set `self.OriginalMaterials` (`MeshComponent.GetMaterials` (`self.Mesh`)))
  (for _array_element (`self.FadeMaterialInstances`)
    (bind _returnvalue (`KismetMaterialLibrary.CreateDynamicMaterialInstance` _array_element))
    (`KismetArrayLibrary.Array_AddUnique` (`self.Dynamic Material Instance`) _returnvalue)))