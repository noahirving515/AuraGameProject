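; BP_SlingshotRock is a rock actor in the enemy abilities folder that tumbles randomly, giving a slingshot rock a spinning look.
; BeginPlay picks a random signed rate for yaw, roll and pitch, so each instance spins differently.
; Tick applies those rates, scaled by delta seconds, as a local rotation on the SlingshotRock component for frame-rate independent motion.
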(event `self.ReceiveBeginPlay`
  (bind _returnvalue (`KismetMathLibrary.RandomFloatInRange` -500.0 500.0))
  ; Create random rotator variables (X, Y, Z)
  (set `self.Yaw Rotation Rate` _returnvalue)
  (set `self.Roll Rotation Rate` _returnvalue)
  (set `self.Pitch Rotation Rate` _returnvalue))

(event `self.ReceiveTick`
  (params (DeltaSeconds :type "Float (single-precision)"))
  ; set random rotation on the rock mesh
  (`SceneComponent.K2_AddLocalRotation` (`self.SlingshotRock`) (`KismetMathLibrary.MakeRotator` (* (`self.Roll Rotation Rate`) DeltaSeconds) (* (`self.Pitch Rotation Rate`) DeltaSeconds) (* (`self.Yaw Rotation Rate`) DeltaSeconds)) false false))

(fn `UserConstructionScript`)